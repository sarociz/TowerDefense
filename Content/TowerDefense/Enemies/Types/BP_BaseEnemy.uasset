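; Base enemy for the tower defense game that walks to a goal and damages the player's side through the game mode.
; On BeginPlay it registers with GM_TowerDefense and stores its movement speed; once possessed, it has AIC_Enemy move it to Goal a tick later.
; Incoming hits either reduce life or, with a positive slow value, only set walk speed.
; DealDamage reports damage to the game mode, while death awards money; both destroy the actor.
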(event `self.ReceivePossessed`
  (params (NewController :type "Controller Object Reference"))
  (bind _asaic_enemy (cast `/Game/TowerDefense/Enemies/AIC_Enemy` NewController))
  (set `self.AIController` _asaic_enemy)
  (`KismetSystemLibrary.DelayUntilNextTick`)
  (`/Game/TowerDefense/Enemies/AIC_Enemy.MoveToDestination` (`self.AIController`) (`self.Goal`)))

(event `self.ReceiveBeginPlay`
  (bind _asgm_tower_defense (cast `/Game/TowerDefense/GM_TowerDefense` (`GameplayStatics.GetGameMode`)))
  (bind _output_get (set `self.GMTowerRef` _asgm_tower_defense))
  (`/Game/TowerDefense/GM_TowerDefense.Add Enemy` _output_get)
  (set `self.Slow` (`MovementComponent.GetMaxSpeed` (`self.CharacterMovement`))))

(fn `Dead`
  (`/Game/TowerDefense/GM_TowerDefense.Add Money` (`self.GMTowerRef`) (`self.Money`))
  (`self.K2_DestroyActor`))

(fn `DealDamage`
  (`/Game/TowerDefense/GM_TowerDefense.Receive Damage` (`self.GMTowerRef`) (`self.Damage`))
  (`self.K2_DestroyActor`))

(fn `ReceiveDamage`
  (params (Damage :type Integer) (Slow :type Integer))
  (if (<= Slow 0)
    (bind _output_get (set `self.Life` (- (`self.Life`) Damage 0)))
    (if (<= _output_get 0)
      (`self.Dead`))
    (else
      (set `CharacterMovementComponent.MaxWalkSpeed` (- (`self.Slow`) Slow) (`self.CharacterMovement`)))))

(fn `UserConstructionScript`)