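; Base enemy for the tower defense game that travels to a goal, can be killed for money and can damage the player's side.
; On possession it stores its AIC_Enemy controller, waits a tick, then has it move to Goal; on BeginPlay it registers with GM_TowerDefense.
; ReceiveDamage lowers Life and, at zero or below, awards Money through the game mode and destroys the enemy.
; DealDamage passes its Damage to the game mode, then destroys the enemy.
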(event `self.ReceivePossessed`
  (params (NewController :type "Controller Object Reference"))
  (bind _asaic_enemy (cast `/Game/TowerDefense/Enemies/AIC_Enemy` NewController))
  (set `self.AIController` _asaic_enemy)
  (`KismetSystemLibrary.DelayUntilNextTick`)
  (`/Game/TowerDefense/Enemies/AIC_Enemy.MoveToDestination` (`self.AIController`) (`self.Goal`)))

(event `self.ReceiveBeginPlay`
  (bind _asgm_tower_defense (cast `/Game/TowerDefense/GM_TowerDefense` (`GameplayStatics.GetGameMode`)))
  (bind _output_get (set `self.GM Tower Defense` _asgm_tower_defense))
  (`/Game/TowerDefense/GM_TowerDefense.Add Enemy` _output_get))

(fn `DealDamage`
  (`/Game/TowerDefense/GM_TowerDefense.Receive Damage` (`self.GM Tower Defense`) (`self.Damage`))
  (`self.K2_DestroyActor`))

(fn `ReceiveDamage`
  (params (Damage :type Integer))
  (bind _output_get (set `self.Life` (- (`self.Life`) Damage)))
  (if (<= _output_get 0)
    (bind _asgm_tower_defense (cast `/Game/TowerDefense/GM_TowerDefense` (`GameplayStatics.GetGameMode`)))
    (`/Game/TowerDefense/GM_TowerDefense.Add Money` _asgm_tower_defense (`self.Money`))
    (`self.K2_DestroyActor`)))

(fn `UserConstructionScript`)