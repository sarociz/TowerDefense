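; Tower defense spawner that registers with GM_TowerDefense and spawns enemies at its own transform, each given the Destination's location as its Goal.
; EnemyRounds holds rounds of waves, each defining enemy type, count and spawn interval.
; A looping timer spawns each wave, then moves straight on to the next.
; A finished round calls SetIsEndWave on the game mode; exhausting all rounds calls SetIsEndRound.
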(event `self.ReceiveBeginPlay`
  (bind _asgm_tower_defense (cast `/Game/TowerDefense/GM_TowerDefense` (`GameplayStatics.GetGameMode`)))
  (`/Game/TowerDefense/GM_TowerDefense.SetSpawnerRef` _asgm_tower_defense self))

(event `Start Round`
  (if (not (> (`self.nRound`) (`KismetArrayLibrary.Array_Length` (`self.EnemyRounds`))))
    (`self.Event Array`)))

(event `Event Array`
  (if (`KismetArrayLibrary.Array_IsValidIndex` (`self.Get Waves`) (`self.nWave`))
    (bind _returnvalue (`KismetSystemLibrary.K2_SetTimerDelegate` (delegate `Event Spawn`) (`self.GetWaveTimer`) true))
    (set `self.SpawnTimeHandle` _returnvalue)
    (else
      (`KismetSystemLibrary.K2_ClearAndInvalidateTimerHandle` (`self.SpawnTimeHandle`) :!label _label)
      (set `self.nWave` (+ (`self.nWave`) 1))
      (if (`KismetArrayLibrary.Array_IsValidIndex` (`self.Get Waves`) (`self.nWave`))
        (`self.Event Array`)
        (set `self.ActualEnemies` 0)
        (else
          (bind _result (`/Engine/EditorBlueprintResources/StandardMacros.IncrementInt` (`self.nRound`))
            (:`  `
              (if (`KismetArrayLibrary.Array_IsValidIndex` (`self.EnemyRounds`) _result)
                (set `self.nWave` 0)
                (set `self.ActualEnemies` 0)
                (bind _asgm_tower_defense (cast `/Game/TowerDefense/GM_TowerDefense` (`GameplayStatics.GetGameMode`)))
                (`/Game/TowerDefense/GM_TowerDefense.Set isEndWave` _asgm_tower_defense)
                (else
                  (`KismetSystemLibrary.PrintString` "NO MORE ROUNDSSSS" true true (struct :`G` 1.0 :`B` 0.144892 :`A` 1.0) 5.0)
                  (bind _asgm_tower_defense_2 (cast `/Game/TowerDefense/GM_TowerDefense` (`GameplayStatics.GetGameMode`)))
                  (`/Game/TowerDefense/GM_TowerDefense.Set isEndRound` _asgm_tower_defense_2))))))))))

(event `Event Spawn`
  (if (>= (`self.ActualEnemies`) (`self.GetEnemies`))
    (goto _label)
    (else
      (bind _returnvalue (`|SpawnActorFromClass` (`self.GetEnemyType`) (`self.GetTransform`) "AdjustIfPossibleButAlwaysSpawn" "MultiplyWithRoot" null null))
      (set `/Game/TowerDefense/Enemies/BP_BaseEnemy.Goal` (`SceneComponent.K2_GetComponentLocation` (`self.Destination`)) _returnvalue)
      (set `self.ActualEnemies` (+ (`self.ActualEnemies`) 1)))))

(fn `Get Waves`
  (returns (`Actual Wave` :type "Array of /Game/TowerDefense/Enemies/S_EnemyWave Structure"))
  (bind _output_round (break `/Game/TowerDefense/Enemies/S_EnemyRounds` (`|GetArrayItem` (`self.EnemyRounds`) (`self.nRound`))))
  (return _output_round))

(fn `GetEnemies`
  (returns (`Num Enemies` :type Integer))
  (bind _output_numenemies (break `/Game/TowerDefense/Enemies/S_EnemyWave` (`|GetArrayItem` (`self.Get Waves`) (`self.nWave`))))
  (return _output_numenemies))

(fn `GetEnemyType`
  (returns (`Enemy Type` :type "/Game/TowerDefense/Enemies/BP_BaseEnemy Class Reference"))
  (bind (_output_numenemies _output_enemytype) (break `/Game/TowerDefense/Enemies/S_EnemyWave` (`|GetArrayItem` (`self.Get Waves`) (`self.nWave`))))
  (return _output_enemytype))

(fn `GetWaveTimer`
  (returns (`Wave Timer` :type "Float (double-precision)"))
  (bind (_output_numenemies _output_enemytype _output_wavetimer) (break `/Game/TowerDefense/Enemies/S_EnemyWave` (`|GetArrayItem` (`self.Get Waves`) (`self.nWave`))))
  (return _output_wavetimer))

(fn `UserConstructionScript`)