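; Tower defense player that handles mouse-driven turret placement, using the game mode for placement state and money checks.
; In placement mode it spawns a BP_BuildTurret preview, which a looping timer moves to the cursor's line-trace hit while checking validity.
; A left click checks the HUD button's cost against available money, then replaces a valid preview with a BP_BasicTurret and ends placement.
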(event `self.ReceiveBeginPlay`
  (set `PlayerController.bShowMouseCursor` true (`GameplayStatics.GetPlayerController` 0))
  (bind _asgm_tower_defense (cast `/Game/TowerDefense/GM_TowerDefense` (`GameplayStatics.GetGameMode`)))
  (bind _output_get (set `self.GMTowerRef` _asgm_tower_defense))
  (`/Game/TowerDefense/GM_TowerDefense.SetPlayerRef` _output_get self))

(event `Key|LeftMouseButton`
  (params (Key :type "Key Structure"))
  (:`Pressed`
    (bind _canbuy (`/Game/TowerDefense/GM_TowerDefense.HasMuuney` (`self.GMTowerRef`) (`self.Get Cost`)))
    (if _canbuy
      (`KismetSystemLibrary.PrintString` "Colocando turret" true true (struct :`R` 0.095818 :`G` 1.0 :`B` 0.082046 :`A` 1.0))
      (if (`self.Get IsActivePlacement`)
        (`self.PlaceTurret`))
      (else
        (`KismetSystemLibrary.PrintString` "No tienes dinero" true true (struct :`R` 1.0 :`G` 0.244628 :`B` 0.704256 :`A` 1.0) 5.0)))))

(event `DebugRaycast`
  (params (Start :type "Vector Structure") (Direction :type "Vector Structure"))
  (bind (_outhit _returnvalue) (`KismetSystemLibrary.LineTraceSingle` :`Start` Start :`End` Direction :`TraceChannel` "TraceTypeQuery1" :`bTraceComplex` true :`DrawTime` 100.0))
  (if _returnvalue
    (`|SpawnActorFromClass` "/Game/TowerDefense/Turret/BP_BasicTurret.BP_BasicTurret_C" (`KismetMathLibrary.MakeTransform` (`.Location` (`GameplayStatics.BreakHitResult` _outhit))) "Undefined" "MultiplyWithRoot" null null)
    (`self.Set IsActivePlacement` false)
    (`self.K2_DestroyActor` (`self.TurretPlace`))))

(event `PlaceTurret`
  (bind _turretplace (`self.TurretPlace`))
  (if (and (`self.Get IsActivePlacement`) (`/Game/TowerDefense/Turret/BP_BuildTurret.CanPlace?` _turretplace))
    (`|SpawnActorFromClass` "/Game/TowerDefense/Turret/BP_BasicTurret.BP_BasicTurret_C" (`self.GetTransform` _turretplace) "AlwaysSpawn" "MultiplyWithRoot" null null)
    (`self.Set IsActivePlacement` false)
    (`self.K2_DestroyActor` (`self.TurretPlace`))
    (`/Game/TowerDefense/HUD/WBP_Button.Set Buy ButtonText` (`/Game/TowerDefense/HUD/WBP_HUD.WBP_Button` (`/Game/TowerDefense/GM_TowerDefense.HUD` (`self.GMTowerRef`))))))

(event `Placement Mode`
  (if (`self.Get IsActivePlacement`)
    (bind _returnvalue (`|SpawnActorFromClass` "/Game/TowerDefense/Turret/BP_BuildTurret.BP_BuildTurret_C" (`KismetMathLibrary.MakeTransform` (`self.Get PlayerPos`)) "Undefined" "MultiplyWithRoot" null null))
    (set `self.TurretPlace` _returnvalue)
    (if (`KismetSystemLibrary.K2_IsValidTimerHandle` (`self.TurretPlaceTimerHandle`))
      (`KismetSystemLibrary.K2_UnPauseTimerHandle` (`self.TurretPlaceTimerHandle`))
      (else
        (bind _returnvalue_2 (`KismetSystemLibrary.K2_SetTimerDelegate` (delegate `Placing Turret`) 0.01 true))
        (set `self.TurretPlaceTimerHandle` _returnvalue_2)))))

(event `Placing Turret`
  (bind (_start _end) (`self.Get PlayerPos`))
  (bind _turretplace (`self.TurretPlace`))
  (bind _turretplace_2 (`self.TurretPlace`))
  (if (`self.Get IsActivePlacement`)
    (bind (_outhit _returnvalue) (`KismetSystemLibrary.LineTraceSingle` :`Start` _start :`End` _end :`TraceChannel` "TraceTypeQuery1" :`DrawTime` 100.0))
    (if _returnvalue
      (`/Engine/EditorBlueprintResources/StandardMacros.IsValid` _turretplace
        (:`Is Valid`
          (`/Game/TowerDefense/Turret/BP_BuildTurret.CheckPlacement` (`self.TurretPlace`))
          (`self.K2_SetActorLocation` _turretplace (`.ImpactPoint` (`GameplayStatics.BreakHitResult` _outhit)) false true))))
    (else
      (`KismetSystemLibrary.K2_PauseTimerHandle` (`self.TurretPlaceTimerHandle`))
      (`/Engine/EditorBlueprintResources/StandardMacros.IsValid` _turretplace_2
        (:`Is Valid`
          (`self.K2_DestroyActor` _turretplace_2))))))

(fn `Get Cost`
  (returns (Cost :type Integer))
  (return (`/Game/TowerDefense/HUD/WBP_Button.Cost` (`/Game/TowerDefense/HUD/WBP_HUD.WBP_Button` (`/Game/TowerDefense/GM_TowerDefense.HUD` (`self.GMTowerRef`))))))

(fn `Get IsActivePlacement`
  (returns (isActivePlacement :type Boolean))
  (return (`/Game/TowerDefense/GM_TowerDefense.isActivePlacement` (`self.GMTowerRef`))))

(fn `Get PlayerPos`
  (returns (Start :type "Vector Structure") (End :type "Vector Structure"))
  (bind (_worldlocation _worlddirection) (`PlayerController.DeprojectMousePositionToWorld` (`GameplayStatics.GetPlayerController` 0)))
  (return _worldlocation (+ _worldlocation (* _worlddirection 3000.0))))

(fn `Set IsActivePlacement`
  (params (IsActive :type Boolean))
  (`/Game/TowerDefense/GM_TowerDefense.Set IsActivePlacement` (`self.GMTowerRef`) IsActive))

(fn `UserConstructionScript`)