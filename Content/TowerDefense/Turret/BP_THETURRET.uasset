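; Tower defense turret that fires once at enemies entering its detection area, then destroys itself.
; Overlap events maintain a list of BP_BaseEnemy actors inside the area.
; An enemy entering starts a three-second delay, after which a projectile spawns at the shooting point, homing on the first listed enemy's capsule.
; The turret directly damages every listed enemy without slow, independent of projectile impact, before removing itself.
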(event `self.DetectionArea.OnComponentBeginOverlap`
  (params (OverlappedComponent :type "PrimitiveComponent Object Reference") (OtherActor :type "Actor Object Reference") (OtherComp :type "PrimitiveComponent Object Reference") (OtherBodyIndex :type Integer) (bFromSweep :type Boolean) (SweepResult :type "HitResult Structure (by ref)"))
  (bind _enemiesinarea (`self.EnemiesInArea`))
  (bind _asbp_base_enemy (cast `/Game/TowerDefense/Enemies/Types/BP_BaseEnemy` OtherActor))
  (`KismetArrayLibrary.Array_Add` (`self.EnemiesInArea`) _asbp_base_enemy)
  (`KismetSystemLibrary.Delay` 3.0)
  (bind _returnvalue (`|SpawnActorFromClass` (`self.THEPROJECTILE`) (`SceneComponent.K2_GetComponentToWorld` (`self.Shooting Point`)) "AdjustIfPossibleButAlwaysSpawn" "MultiplyWithRoot" null null))
  (set `ProjectileMovementComponent.HomingTargetComponent` (`Character.CapsuleComponent` (`|GetArrayItem` _enemiesinarea)) (`/Game/TowerDefense/Turret/BP_THEPROJECTILE.ProjectileMovement` _returnvalue))
  (for _array_element _enemiesinarea
    (`/Game/TowerDefense/Enemies/Types/BP_BaseEnemy.ReceiveDamage` _array_element (`self.Damage`) 0))
  (`self.K2_DestroyActor`))

(event `self.DetectionArea.OnComponentEndOverlap`
  (params (OverlappedComponent :type "PrimitiveComponent Object Reference") (OtherActor :type "Actor Object Reference") (OtherComp :type "PrimitiveComponent Object Reference") (OtherBodyIndex :type Integer))
  (bind _asbp_base_enemy (cast `/Game/TowerDefense/Enemies/Types/BP_BaseEnemy` OtherActor))
  (`KismetArrayLibrary.Array_RemoveItem` (`self.EnemiesInArea`) _asbp_base_enemy))

(fn `UserConstructionScript`)