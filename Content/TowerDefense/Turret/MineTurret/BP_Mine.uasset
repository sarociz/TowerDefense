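; BP_Mine is a tower defense mine that triggers when a BP_BaseEnemy enters its DetectionArea.
; Overlap events add and remove enemies in a tracked array.
; An enemy entering starts a configurable delay, after which the mine loops over the tracked enemies and destroys itself.
; The loop body is empty: the ReceiveDamage call is disconnected, so the mine deals no damage as wired.
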(event `self.DetectionArea.OnComponentBeginOverlap`
  (params (OverlappedComponent :type "PrimitiveComponent Object Reference") (OtherActor :type "Actor Object Reference") (OtherComp :type "PrimitiveComponent Object Reference") (OtherBodyIndex :type Integer) (bFromSweep :type Boolean) (SweepResult :type "HitResult Structure (by ref)"))
  (bind _asbp_base_enemy (cast `/Game/TowerDefense/Enemies/Types/BP_BaseEnemy` OtherActor))
  (`KismetArrayLibrary.Array_Add` (`self.EnemiesInArea_0`) _asbp_base_enemy)
  (`KismetSystemLibrary.Delay` (`self.WaitExplosionTime`))
  (for _array_element (`self.EnemiesInArea_0`)
    _)
  (`self.K2_DestroyActor`))

(event `self.DetectionArea.OnComponentEndOverlap`
  (params (OverlappedComponent :type "PrimitiveComponent Object Reference") (OtherActor :type "Actor Object Reference") (OtherComp :type "PrimitiveComponent Object Reference") (OtherBodyIndex :type Integer))
  (bind _asbp_base_enemy (cast `/Game/TowerDefense/Enemies/Types/BP_BaseEnemy` OtherActor))
  (`KismetArrayLibrary.Array_RemoveItem` (`self.EnemiesInArea_0`) _asbp_base_enemy))

(fn `UserConstructionScript`)