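; Tower defense turret that fires homing projectiles at flying BP_Archaeopteryx enemies inside its detection area.
; Overlap events maintain the FlyingInArea list; each Archaeopteryx entry fires immediately and sets a looping timer at the rate of fire.
; Each shot spawns a projectile at the shooting point, homing on the first listed target's capsule and carrying the turret's damage.
; Any other overlapping actor clears InScope, pausing fire; an emptied list also clears the timer.
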(event `self.DetectionArea.OnComponentBeginOverlap`
  (params (OverlappedComponent :type "PrimitiveComponent Object Reference") (OtherActor :type "Actor Object Reference") (OtherComp :type "PrimitiveComponent Object Reference") (OtherBodyIndex :type Integer) (bFromSweep :type Boolean) (SweepResult :type "HitResult Structure (by ref)"))
  (bind _asbp_archaeopteryx (cast `/Game/TowerDefense/Enemies/Types/BP_Archaeopteryx` OtherActor)
    (:`then`
      (`KismetArrayLibrary.Array_Add` (`self.Flying in Area`) _asbp_archaeopteryx)
      (set `self.inScope` true))
    (:`CastFailed`
      (set `self.inScope` false)))
  (if (`self.inScope`)
    (bind _returnvalue (`KismetSystemLibrary.K2_SetTimerDelegate` (delegate `Shoot`) (`self.Rate of Fire`) true))
    (set `self.Shoot timer Handle_0` _returnvalue)
    (if (`self.inScope`)
      (`self.Shoot`))))

(event `Shoot`
  (if (`self.inScope`)
    (bind _returnvalue (`|SpawnActorFromClass` (`self.FlyingProjectile`) (`SceneComponent.K2_GetComponentToWorld` (`self.Shooting Point`)) "AdjustIfPossibleButAlwaysSpawn" "MultiplyWithRoot" null null))
    (if (`self.inScope`)
      (set `ProjectileMovementComponent.HomingTargetComponent` (`Character.CapsuleComponent` (`|GetArrayItem` (`self.Flying in Area`))) (`/Game/TowerDefense/Turret/BP_TurretProjectile.ProjectileMovement` _returnvalue))
      (set `/Game/TowerDefense/Turret/BP_TurretProjectile.Damage` (`self.Damage`) _returnvalue))))

(event `self.DetectionArea.OnComponentEndOverlap`
  (params (OverlappedComponent :type "PrimitiveComponent Object Reference") (OtherActor :type "Actor Object Reference") (OtherComp :type "PrimitiveComponent Object Reference") (OtherBodyIndex :type Integer))
  (bind _flying_in_area (`self.Flying in Area`))
  (bind _asbp_archaeopteryx (cast `/Game/TowerDefense/Enemies/Types/BP_Archaeopteryx` OtherActor))
  (`KismetArrayLibrary.Array_RemoveItem` _flying_in_area _asbp_archaeopteryx)
  (if (`KismetArrayLibrary.Array_IsEmpty` _flying_in_area)
    (`KismetSystemLibrary.K2_ClearAndInvalidateTimerHandle` (`self.Shoot timer Handle_0`))
    (set `self.inScope` false)))

(fn `UserConstructionScript`)