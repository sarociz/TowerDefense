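; Basic tower defense turret that fires homing projectiles at enemies inside its detection area, ignoring Archaeopteryx enemies as targets.
; Overlap events maintain the enemy list, and each valid entry fires at once and sets a looping timer at the fire rate.
; Each shot homes on the first listed enemy's capsule and receives the turret's damage value.
; The timer is cleared when the list empties.
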(event `self.DetectionArea.OnComponentBeginOverlap`
  (params (OverlappedComponent :type "PrimitiveComponent Object Reference") (OtherActor :type "Actor Object Reference") (OtherComp :type "PrimitiveComponent Object Reference") (OtherBodyIndex :type Integer) (bFromSweep :type Boolean) (SweepResult :type "HitResult Structure (by ref)"))
  (bind _asbp_base_enemy (cast `/Game/TowerDefense/Enemies/Types/BP_BaseEnemy` OtherActor))
  (cast `/Game/TowerDefense/Enemies/Types/BP_Archaeopteryx` _asbp_base_enemy
    (:`then`
      (set `self.isShooting` false))
    (:`CastFailed`
      (set `self.isShooting` true)
      (`KismetArrayLibrary.Array_Add` (`self.EnemiesInArea`) _asbp_base_enemy)
      (if (`self.isShooting`)
        (bind _returnvalue (`KismetSystemLibrary.K2_SetTimerDelegate` (delegate `Shoot`) (`self.Rate of Fire`) true))
        (set `self.Shoot timer Handle` _returnvalue)
        (`self.Shoot`)))))

(event `Shoot`
  (bind _returnvalue (`|SpawnActorFromClass` (`self.Projectile`) (`SceneComponent.K2_GetComponentToWorld` (`self.Shooting Point`)) "AdjustIfPossibleButAlwaysSpawn" "MultiplyWithRoot" null null))
  (set `ProjectileMovementComponent.HomingTargetComponent` (`Character.CapsuleComponent` (`|GetArrayItem` (`self.EnemiesInArea`))) (`/Game/TowerDefense/Turret/BP_TurretProjectile.ProjectileMovement` _returnvalue))
  (set `/Game/TowerDefense/Turret/BP_TurretProjectile.Damage` (`self.Damage`) _returnvalue))

(event `self.DetectionArea.OnComponentEndOverlap`
  (params (OverlappedComponent :type "PrimitiveComponent Object Reference") (OtherActor :type "Actor Object Reference") (OtherComp :type "PrimitiveComponent Object Reference") (OtherBodyIndex :type Integer))
  (bind _enemiesinarea (`self.EnemiesInArea`))
  (bind _asbp_base_enemy (cast `/Game/TowerDefense/Enemies/Types/BP_BaseEnemy` OtherActor))
  (`KismetArrayLibrary.Array_RemoveItem` _enemiesinarea _asbp_base_enemy)
  (if (`KismetArrayLibrary.Array_IsEmpty` _enemiesinarea)
    (`KismetSystemLibrary.K2_ClearAndInvalidateTimerHandle` (`self.Shoot timer Handle`))
    (set `self.isShooting` false)))

(fn `UserConstructionScript`)