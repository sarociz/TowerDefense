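; Tower defense game mode, judging by its name, that tracks player health and money.
; BeginPlay prints a debug note and calls ReceiveDamage and AddMoney with zero.
; ReceiveDamage subtracts from HealthPoints and prints a death message at zero or below, without calling LoseGame.
; LoseGame pauses and prints defeat, while AddMoney updates and prints the Money total.
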(event `self.ReceiveBeginPlay`
  (`KismetSystemLibrary.PrintString` "CREATE INTERFAZ \n \n \ntiene un return")
  (`self.Receive Damage` 0)
  (`self.Add Money` 0))

(fn `Add Money`
  (params (Money :type Integer))
  (set `self.Money` (+ (`self.Money`) Money))
  (`KismetSystemLibrary.PrintString` (`KismetStringLibrary.Conv_IntToString` (`self.Money`)) true true (struct :`R` 1.0 :`G` 0.790188 :`B` 0.007983 :`A` 1.0)))

(fn `Lose Game`
  (`GameplayStatics.SetGamePaused` true)
  (`KismetSystemLibrary.PrintString` "Defeated"))

(fn `Receive Damage`
  (params (Damage :type Integer))
  (bind _output_get (set `self.Health Points` (- (`self.Health Points`) Damage)))
  (if (<= _output_get 0)
    (`KismetSystemLibrary.PrintString` "Has muerto")))

(fn `UserConstructionScript`)